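; Checkpoint actor that saves the player's position when the ThirdPersonCharacter overlaps its Box trigger.
; It loads the CheckPointSlot save, or creates a CheckPoint save object if none exists, then writes the character's location to LastLocation and saves it.
; After saving, it swaps the Checkpoint component's template to CheckpointActive to show activation.
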(event `self.Box.OnComponentBeginOverlap`
  (params (OverlappedComponent :type "PrimitiveComponent Object Reference") (OtherActor :type "Actor Object Reference") (OtherComp :type "PrimitiveComponent Object Reference") (OtherBodyIndex :type Integer) (bFromSweep :type Boolean) (SweepResult :type "HitResult Structure (by ref)"))
  (bind _location (`self.Location`))
  (bind _saversubclass (`self.SaverSubClass`))
  (bind _asthird_person_character (cast `/Game/Blueprints/Character/ThirdPersonCharacter` OtherActor))
  (set `self.Location` (`self.K2_GetActorLocation` _asthird_person_character))
  (bind _returnvalue (`GameplayStatics.DoesSaveGameExist` "CheckPointSlot"))
  (if _returnvalue
    (bind _returnvalue_2 (`GameplayStatics.LoadGameFromSlot` "CheckPointSlot"))
    (bind _output_get (set `self.SaverSubClass` _returnvalue_2))
    (bind _ascheck_point (cast `/Game/UI_Menu/CheckPoint` _output_get))
    (set `/Game/UI_Menu/CheckPoint.LastLocation` _location _ascheck_point)
    (bind _returnvalue_3 (`GameplayStatics.SaveGameToSlot` _saversubclass "CheckPointSlot"))
    (else
      (bind _returnvalue_4 (`GameplayStatics.CreateSaveGameObject` "/Game/UI_Menu/CheckPoint.CheckPoint_C"))
      (bind _output_get_2 (set `self.SaverSubClass` _returnvalue_4))
      (bind _ascheck_point_2 (cast `/Game/UI_Menu/CheckPoint` _output_get_2))
      (set `/Game/UI_Menu/CheckPoint.LastLocation` _location _ascheck_point_2)
      (bind _returnvalue_5 (`GameplayStatics.SaveGameToSlot` _saversubclass "CheckPointSlot"))))
  (`ParticleSystemComponent.SetTemplate` (`self.Checkpoint`) (`self.CheckpointActive`)))

(fn `UserConstructionScript`)