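; Test grappling hook actor that pulls the player toward itself when spawned.
; On BeginPlay it attaches its Cable end to the player pawn, then after a brief delay launches the ThirdPersonCharacter along the vector to its Sphere, overriding velocity.
; Launch strength scales with distance and one frame's delta time, and is printed for debugging.
; Two seconds later it decrements the character's WorldPillarCount and destroys itself.
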(event `self.ReceiveBeginPlay`
  (bind _returnvalue (`GameplayStatics.GetPlayerPawn` 0))
  (bind _returnvalue_2 (* (- (`SceneComponent.K2_GetComponentLocation` (`self.Sphere`)) (`self.K2_GetActorLocation` _returnvalue)) (* (`GameplayStatics.GetWorldDeltaSeconds`) 250.0)))
  (`CableComponent.SetAttachEndTo` (`self.Cable`) _returnvalue "None")
  (`KismetSystemLibrary.Delay` 0.1)
  (bind _asthird_person_character (cast `/Game/Blueprints/Character/ThirdPersonCharacter` _returnvalue))
  (`Character.LaunchCharacter` _asthird_person_character _returnvalue_2 true true)
  (`KismetSystemLibrary.PrintString` (`KismetStringLibrary.Conv_VectorToString` _returnvalue_2))
  (`KismetSystemLibrary.Delay` 2.0)
  (`/Engine/EditorBlueprintResources/StandardMacros.DecrementInt` (`/Game/Blueprints/Character/ThirdPersonCharacter.WorldPillarCount` _asthird_person_character)
    (:`  `
      (`self.K2_DestroyActor`))))

(fn `UserConstructionScript`)