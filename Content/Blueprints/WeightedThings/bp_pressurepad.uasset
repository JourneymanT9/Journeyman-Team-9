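; Pressure pad that moves a referenced ActorWeight actor up and down when weighted objects step on or off it.
; Overlaps from actors tagged "weight" raise the target by a fixed vertical offset on begin and lower it by the same offset on end.
; The move is an instant, non-swept relative location change with no overlap counting, so each additional weight shifts the target again.
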(event `self.ReceiveActorBeginOverlap`
  (params (OtherActor :type "Actor Object Reference"))
  (bind _actor_weight (`self.Actor_weight`))
  ;[0 0.22 1] Pressed
  (if (`self.ActorHasTag` OtherActor "weight")
    (`/Engine/EditorBlueprintResources/StandardMacros.IsValid` _actor_weight
      (:`Is Valid`
        ;[0.005835 1 0] Action - ON
        (`self.K2_SetActorLocation` _actor_weight (+ (`self.K2_GetActorLocation` _actor_weight) (0.0 0.0 300.0)) false false)))))

(event `self.ReceiveActorEndOverlap`
  (params (OtherActor :type "Actor Object Reference"))
  (bind _actor_weight (`self.Actor_weight`))
  ;[0 0.2557 1] Released
  (if (`self.ActorHasTag` OtherActor "weight")
    (`/Engine/EditorBlueprintResources/StandardMacros.IsValid` _actor_weight
      (:`Is Valid`
        ;[1 0 0.04868] Action - OFF
        (`self.K2_SetActorLocation` _actor_weight (+ (`self.K2_GetActorLocation` _actor_weight) (0.0 0.0 -300.0)) false false)))))

(fn `UserConstructionScript`)