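; Portal actor that sends the third-person character either to another level or to a named portal in the same level.
; An outer trigger toggles the particles and timeline-faded light, while an inner trigger starts travel, with both also checked on BeginPlay.
; Key/value arrays become an options string: LevelName opens LoadScreen with those options, while PortalName moves the player to the matching portal's spawn point.
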(event OnComponentBeginOverlap(GoToTriggerBox)
  (params (OverlappedComponent :type Primitive%20Component%20Object%20Reference) (OtherActor :type Actor%20Object%20Reference) (OtherComp :type Primitive%20Component%20Object%20Reference) (OtherBodyIndex :type Integer) (bFromSweep :type Boolean) (SweepResult :type Hit%20Result%20Structure%20%28by%20ref%29))
  ;[1 1 1] Takes player to level
  (bind _asthird_person_character (Utilities|Casting|CastToThirdPersonCharacter OtherActor))
  (Portal|PortalHandler _asthird_person_character))

(event OnComponentBeginOverlap(PortalOnTriggerBox)
  (params (OverlappedComponent :type Primitive%20Component%20Object%20Reference) (OtherActor :type Actor%20Object%20Reference) (OtherComp :type Primitive%20Component%20Object%20Reference) (OtherBodyIndex :type Integer) (bFromSweep :type Boolean) (SweepResult :type Hit%20Result%20Structure%20%28by%20ref%29))
  ;[1 1 1] Particles(Portal) On/ Off
  (Utilities|Casting|CastToThirdPersonCharacter OtherActor)
  (Components|Activation|Activate (Variables|Default|GetP_portal) true)
  (CallFunction|TurnonLight))

(event OnComponentEndOverlap(PortalOnTriggerBox)
  (params (OverlappedComponent :type Primitive%20Component%20Object%20Reference) (OtherActor :type Actor%20Object%20Reference) (OtherComp :type Primitive%20Component%20Object%20Reference) (OtherBodyIndex :type Integer))
  ;[1 1 1] Particles(Portal) On/ Off
  (Utilities|Casting|CastToThirdPersonCharacter OtherActor)
  (Components|Activation|Deactivate (Variables|Default|GetP_portal))
  (CallFunction|TurnOffLight))

(event Custom|TurnOnLight
  ;[1 1 1] Light Handler
  (bind _lightscale (Timeline|LightTimeLine Play)
    (:Update
      (Rendering|Components|Light|SetIntensity (Variables|Default|GetPointLight) (* _lightscale 1e+05)))))

(event Custom|TurnOffLight
  ;[1 1 1] Light Handler
  (bind _lightscale (Timeline|LightTimeLine Reverse)
    (:Update
      (Rendering|Components|Light|SetIntensity (Variables|Default|GetPointLight) (* _lightscale 1e+05)))))

(event Custom|TransportedTo
  (params (Player :type Third%20Person%20Character%20Object%20Reference))
  (Transformation|SetActorLocationAndRotation Player (Transformation|GetWorldLocation (Variables|Default|GetPlayerSpawn))))

(event EventBeginPlay
  (bind _returnvalue (Game|Player|GetPlayerPawn 0))
  (bind _p_portal (Variables|Default|GetP_portal))
  ;[1 1 1] Checks to see if the player is overlapping with the GoTo trigger box
  (if (Collision|IsOverlappingActor (Variables|Default|GetGoTo%20Trigger%20Box) _returnvalue :!class /Script/Engine.PrimitiveComponent)
    (bind _asthird_person_character (Utilities|Casting|CastToThirdPersonCharacter _returnvalue))
    (Portal|PortalHandler _asthird_person_character)
    (else
      ;[1 1 1] Checks to see if the player is overlapped with the Portal On Trigger box
      (if (Collision|IsOverlappingActor (Variables|Default|GetPortalOn%20Trigger%20Box) (Game|Player|GetPlayerPawn 0) :!class /Script/Engine.PrimitiveComponent)
        ;[1 1 1] Handle Portal particles
        (Components|Activation|Activate _p_portal true) ; Turn on the particle effect
        ;[1 1 1] handle Portal Light
        (CallFunction|TurnonLight)
        (else
          (Components|Activation|Deactivate _p_portal) ; Turn off the portal particle effect
          (CallFunction|TurnOffLight))))))

(fn ConstructionScript
  (|CallParentFunction))

(fn PortalHandler
  (params (Player :type Third%20Person%20Character%20Object%20Reference))
  (bind _optionstring (Variables|Portal|GetOptionString))
  (Portal|EncodeOptions)
  (if (Class|GameplayStatics|HasOption _optionstring "LevelName")
    (Portal|GotoLevel)
    (elif (Class|GameplayStatics|HasOption _optionstring "PortalName")
      (Portal|GotoPortal Player))))

(fn EncodeOptions
  (for (_array_element _array_index) (Variables|Portal|GetOptionKeys)
    (Variables|Portal|SetOptionString (Utilities|String|Append (Variables|Portal|GetOptionString) "?" _array_element "=" (Utilities|Array|Get(acopy) (Variables|Portal|GetOptions) _array_index)))))

(fn TeleportPlayer
  (params (Portal :type BP%20Portal%20Transition%20Object%20Reference) (Player :type Third%20Person%20Character%20Object%20Reference))
  (Transformation|SetActorLocationAndRotation Player "0, 0, 0" (Transformation|GetActorRotation Portal)))

(fn GotoPortal
  (params (Player :type Third%20Person%20Character%20Object%20Reference))
  (bind _outactors (Actor|GetAllActorsOfClass (Utilities|GetClass self)))
  (bind _array_element (Utilities|Array|ForEachLoopwithBreak _outactors)
    (:LoopBody
      (bind _asbp_portal_transition (Utilities|Casting|CastToBP_Portal_Transition _array_element))
      (if (Utilities|Enum|Equal(Enum) (Variables|BP_Portal_Transition_C|GetPortalName _asbp_portal_transition) (Class|GameplayStatics|ParseOption (Variables|Portal|GetOptionString) "PortalName"))
        (CallFunction|Transportedto _asbp_portal_transition Player)))))

(fn GotoLevel
  (Game|OpenLevel(byName) "LoadScreen" true (Variables|Portal|GetOptionString)))