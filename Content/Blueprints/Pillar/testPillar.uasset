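; Pillar actor that animates upward or downward along its local Z when spawned, then removes itself after a decay delay.
; A timeline height curve, frame time, Scale and TimeScale drive a per-update offset, less a Scale-based amount not adjusted for frame time, while Scale also sets uniform size.
; After the delay it decrements WorldPillarCount on player 0's ThirdPersonCharacter and destroys itself, only if that cast succeeds.
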(event `self.ReceiveBeginPlay`
  (bind _scale (`self.Scale`))
  (bind _scale_2 (`self.Scale`))
  (bind (_direction _pillar_height) (`Timeline|Timeline_1` :!via `PlayFromStart`)
    (:`Update`
      (`self.K2_AddActorLocalOffset` (`KismetMathLibrary.MakeVector` 0.0 0.0 (- (* (/ 1.0 (`self.timeScale`)) (`GameplayStatics.GetWorldDeltaSeconds`) _scale_2 _pillar_height) (* _scale_2 0.1))))
      (`self.SetActorRelativeScale3D` (`KismetMathLibrary.MakeVector` _scale _scale _scale)))
    (:`Finished`
      (`KismetSystemLibrary.Delay` (`self.decayTime`))
      (bind _asthird_person_character (cast `/Game/Blueprints/Character/ThirdPersonCharacter` (`GameplayStatics.GetPlayerCharacter` 0)))
      (`/Engine/EditorBlueprintResources/StandardMacros.DecrementInt` (`/Game/Blueprints/Character/ThirdPersonCharacter.WorldPillarCount` _asthird_person_character)
        (:`  `
          (`self.K2_DestroyActor`))))))

(fn `UserConstructionScript`)