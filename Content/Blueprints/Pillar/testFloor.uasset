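; Test floor actor that serves as a clickable target surface for the player character's pillar and hook abilities.
; While an ability is prepared, Tick keeps a rock particle preview under the hovering cursor, using DoOnce gates, and accumulates capped charge while the mouse is held.
; On release, below the world pillar limit, it spawns either a charge-scaled pillar at the cursor or a hook, based on the character's toggle.
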(event `self.ReceiveActorBeginCursorOver`
  ;[1 1 1] If target is valid surface
  (set `self.hideParticles` false))

(event `self.Cube.OnClicked`
  (params (TouchedComponent :type "PrimitiveComponent Object Reference") (ButtonPressed :type "Key Structure" :default "AnyKey"))
  ;[1 1 1] Charging
  (set `self.charging` true))

(event `self.ReceiveActorEndCursorOver`
  ;[1 1 1] If target is valid surface
  (set `self.hideParticles` true))

(event `self.ReceiveTick`
  (params (DeltaSeconds :type "Float (single-precision)"))
  (bind (_bblockinghit _binitialoverlap _time _location) (`GameplayStatics.BreakHitResult` (`PlayerController.GetHitResultUnderCursorByChannel` (`GameplayStatics.GetPlayerController` 0) "TraceTypeQuery1" true)))
  ;[1 1 1] Is the player targeting?
  ;[1 1 1] Active or inactive
  (if (`/Game/Blueprints/Character/ThirdPersonCharacter.Ability Prepared` (`self.char`))
    (`|ExecutionSequence`
      (:`then_0`
        ;[1 1 1] Charging
        (if (`self.charging`)
          (bind _output_get (set `self.chargePower` (+ (`GameplayStatics.GetWorldDeltaSeconds`) (`self.chargePower`))))
          (`KismetSystemLibrary.PrintString` (`KismetStringLibrary.Conv_DoubleToString` _output_get))
          (if (>= _output_get 3.0)
            (set `self.chargePower` 3.0)
            (set `self.charging` false))))
      (:`then_1`
        (goto _label_3 :!via `Reset`))
      (:`then_2`
        (if (`self.hideParticles`)
          ;[1 1 1] Turn off particles
          (`/Engine/EditorBlueprintResources/StandardMacros.IsValid` (stale _returnvalue)
            (:`Is Valid`
              (`self.K2_DestroyActor` (`self.RockParticles`) :!label _label)
              (`self.K2_DestroyActor` (stale _returnvalue))
              (goto _label_2 :!via `Reset`))
            (:`Is Not Valid`
              (goto _label_2 :!via `Reset`)))
          (else
            (`|ExecutionSequence`
              (:`then_0`
                ;[1 1 1] Turn on particles
                (`/Engine/EditorBlueprintResources/StandardMacros.DoOnce` false :!label _label_2
                  (:`Completed`
                    (bind _returnvalue (`|SpawnActorFromClass` "/Game/Blueprints/Pillar/Rock_Particle_BP.Rock_Particle_BP_C" (`KismetMathLibrary.MakeTransform` (`KismetMathLibrary.MakeVector` (.x _location) (.y _location) (.z _location)) (`SceneComponent.K2_GetComponentRotation` (`self.Cube`)) (1.0 1.0 1.0)) "AlwaysSpawn" "OverrideRootScale"))
                    (set `self.RockParticles` _returnvalue))))
              (:`then_1`
                ;[1 1 1] Update particle position
                (`self.K2_SetActorLocation` _returnvalue (`KismetMathLibrary.MakeVector` (.x _location) (.y _location) (.z _location)) false false)))))))
    (else
      (`/Engine/EditorBlueprintResources/StandardMacros.DoOnce` false :!label _label_3
        (:`Completed`
          (goto _label))))))

(event `self.Cube.OnReleased`
  (params (TouchedComponent :type "PrimitiveComponent Object Reference") (ButtonReleased :type "Key Structure" :default "AnyKey"))
  (bind _chargepower (`self.chargePower`))
  (bind _char (`self.char`))
  (bind _worldpillarcount (`/Game/Blueprints/Character/ThirdPersonCharacter.WorldPillarCount` _char))
  (bind (_bblockinghit _binitialoverlap _time _location) (`GameplayStatics.BreakHitResult` (`PlayerController.GetHitResultUnderCursorByChannel` (`GameplayStatics.GetPlayerController` 0) "TraceTypeQuery1" true)))
  ;[1 1 1] If particles exist and you click
  (`KismetSystemLibrary.PrintString` (`KismetStringLibrary.Concat_StrStr` "Charge:" (`KismetStringLibrary.Conv_DoubleToString` (`self.chargePower`))))
  (set `self.charging` false)
  (if (`/Game/Blueprints/Character/ThirdPersonCharacter.Ability Prepared` (`self.char`))
    ;[1 1 1] If pillar limit already reached, block spawn
    (if (>= _worldpillarcount (`/Game/Blueprints/Character/ThirdPersonCharacter.WorldPillarLimit` _char))
      (`KismetSystemLibrary.PrintString` "GREEDY")
      (else
        ;[1 1 1] Turn off particles
        (`self.K2_DestroyActor` (`self.RockParticles`))
        (set `/Game/Blueprints/Character/ThirdPersonCharacter.Ability Prepared` false (`self.char`))
        (if (`/Game/Blueprints/Character/ThirdPersonCharacter.PillarToggle` _char)
          ;[1 1 1] Spawn pillar
          (bind _returnvalue (`|SpawnActorFromClass` "/Game/Blueprints/Pillar/testPillar.testPillar_C" (`KismetMathLibrary.MakeTransform` (`KismetMathLibrary.MakeVector` (.x _location) (.y _location) (.z _location)) (`SceneComponent.K2_GetComponentRotation` (`self.Cube`)) (1.0 1.0 1.0)) "AdjustIfPossibleButAlwaysSpawn" "OverrideRootScale"))
          (if (< _chargepower 1.0)
            (set `/Game/Blueprints/Pillar/testPillar.Scale` 1.0 _returnvalue)
            (else
              (set `/Game/Blueprints/Pillar/testPillar.Scale` _chargepower _returnvalue)))
          (`/Engine/EditorBlueprintResources/StandardMacros.IncrementInt` _worldpillarcount
            (:`  `
              (set `self.chargePower` 0.0)
              (goto _label_2 :!via `Reset`)))
          (else
            (`KismetSystemLibrary.PrintString` "Hook")
            (bind _returnvalue_2 (`|SpawnActorFromClass` "/Game/Blueprints/testHook.testHook_C" (`KismetMathLibrary.MakeTransform` (`self.K2_GetActorLocation` (`GameplayStatics.GetPlayerCharacter` 0)) (struct) (1.0 1.0 1.0)) "Undefined" "OverrideRootScale"))
            (`SceneComponent.K2_SetWorldLocation` (`/Game/Blueprints/testHook.Sphere` _returnvalue_2) (`KismetMathLibrary.MakeVector` (.x _location) (.y _location) (.z _location)) false false)))))))

(event `self.ReceiveBeginPlay`
  ;[1 1 1] Enable Input, set character as variable
  (`self.EnableInput` (`GameplayStatics.GetPlayerController` 0))
  (bind _asthird_person_character (cast `/Game/Blueprints/Character/ThirdPersonCharacter` (`GameplayStatics.GetPlayerCharacter` 0)))
  (set `self.char` _asthird_person_character))

(fn `UserConstructionScript`)