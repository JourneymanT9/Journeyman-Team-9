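; Spline rail camera that follows and faces the player pawn while active, using paired player and camera splines.
; Each tick, a recursive bisection search approximates the player's closest time on PlayerSpline.
; That time is eased, or snapped on large differences, then sampled on CameraSpline as the camera's interpolated target.
; The construction script previews the camera at CameraDebugTime, with optional point numbers and runtime debug spheres.
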(event EventTick
  (params (DeltaSeconds :type Float%20%28single-precision%29))
  ;[1 1 1] Update
  (|UpdateGroup DeltaSeconds))

(fn ConstructionScript
  (DebugTools|ScrubCameraTime)
  (DebugTools|SetupDebugNumbers))

(fn UpdateCamera
  (Transformation|SetWorldLocationAndRotation (Variables|Camera|GetCamera) (Math|Interpolation|VInterpTo (Transformation|GetWorldLocation (Variables|Camera|GetCamera)) (Variables|Camera|GetCameraDesiredLocation) (Variables|Default|GetDeltaTime) (Variables|Camera|GetCameraInterpSpeed)) (Math|Rotator|FindLookatRotation (Transformation|GetWorldLocation (Variables|Camera|GetCamera)) (Transformation|GetActorLocation (Variables|Default|GetPlayerPawn))) false false))

(fn ActivateCamera
  (params (Player :type Pawn%20Object%20Reference))
  (Utilities|IsValid Player
    (:Is%20Valid
      (bind _output_get (Variables|Default|SetPlayerPawn Player))
      (bind _asplay_controller (Utilities|Casting|CastToPlayController (Pawn|GetController _output_get)))
      (Variables|Default|SetController _asplay_controller))))

(fn DeactivateCamera
  (Variables|Default|SetPlayerPawn 0))

(fn SetupDebugNumbers
  (if (Variables|DebugTools|GetShowDebug)
    (Utilities|FlowControl|Sequence
      (:then_0
        (DebugTools|AddSplineNumbers (Variables|Spline|GetPlayerSpline)))
      (:then_1
        (DebugTools|AddSplineNumbers (Variables|Spline|GetCameraSpline))))))

(fn AddSplineNumbers
  (params (Spline :type Spline%20Component%20Object%20Reference))
  (for _index (range 0 (- (Spline|GetNumberOfSplinePoints Spline) 1))
    (LocalVariables|Setindex _index)
    (bind _returnvalue (AddComponent|AddTextRenderComponent false (Math|Transform|MakeTransform (+ (.Location (Spline|GetLocationandTangentatSplinePoint Spline _index "Local")) "0, 0,20.000000") (Math|Rotator|CombineRotators (Math|Rotator|MakeRotfromX (.Tangent (Spline|GetLocationandTangentatSplinePoint Spline _index "Local"))) "0,180.000000, 0"))))
    (Rendering|Components|TextRender|SetText _returnvalue (Utilities|Text|ToText(Integer) (LocalVariables|Getindex)))))

(fn DebugSplineMovement
  (if (Variables|DebugTools|GetShowDebug)
    (DebugTools|DrawSplineDebug (Variables|Spline|GetPlayerSpline) (Variables|Spline|GetSplineCurrentTime) (Variables|Spline|GetConstantVelocity) "(R=1.000000,G=0.000000,B=0.000000,A=1.000000)")
    (DebugTools|DrawSplineDebug (Variables|Spline|GetPlayerSpline) (Variables|Spline|GetSplineDesiredTime) (Variables|Spline|GetConstantVelocity) "(R=1.000000,G=0.000000,B=0.000000,A=1.000000)")
    (DebugTools|DrawSplineDebug (Variables|Spline|GetCameraSpline) (Variables|Spline|GetSplineCurrentTime) (Variables|Spline|GetConstantVelocity) "(R=0.000000,G=0.000000,B=1.000000,A=1.000000)")
    (DebugTools|DrawSplineDebug (Variables|Spline|GetCameraSpline) (Variables|Spline|GetSplineDesiredTime) (Variables|Spline|GetConstantVelocity) "(R=0.000000,G=0.000000,B=1.000000,A=1.000000)")))

(fn ScrubCameraTime
  (bind _cameraspline (Variables|Spline|GetCameraSpline))
  (bind _cameradebugtime (Variables|DebugTools|GetCameraDebugTime))
  (bind _constantvelocity (Variables|Spline|GetConstantVelocity))
  (bind _playerspline (Variables|Spline|GetPlayerSpline))
  (bind _returnvalue (Spline|GetLocationatTime _playerspline _cameradebugtime "World" _constantvelocity))
  (bind _returnvalue_2 (Spline|GetLocationatTime _cameraspline _cameradebugtime "World" _constantvelocity))
  (bind _returnvalue_3 (Math|Rotator|FindLookatRotation _returnvalue_2 _returnvalue))
  (bind (_roll _pitch _yaw) (Math|Rotator|BreakRotator _returnvalue_3))
  (Transformation|SetWorldLocationAndRotation (Variables|Camera|GetCamera) _returnvalue_2 (Math|Rotator|MakeRotator 0.0 _pitch _yaw) false false))

(fn RecursiveDistanceCheck
  (params (Iteration :type Integer) (StartTime :type Float%20%28single-precision%29) (EndTime :type Float%20%28single-precision%29))
  (bind _constantvelocity (Variables|Spline|GetConstantVelocity))
  (bind _playerpawn (Variables|Default|GetPlayerPawn))
  (bind _playerspline (Variables|Spline|GetPlayerSpline))
  (bind _returnvalue (Transformation|GetActorLocation _playerpawn))
  (LocalVariables|SetNum Iteration)
  (LocalVariables|SetStart StartTime)
  (LocalVariables|SetEnd EndTime)
  (LocalVariables|SetStartDistance (Math|Vector|VectorLength (- (Spline|GetLocationatTime _playerspline (LocalVariables|GetStart) "World" _constantvelocity) _returnvalue)))
  (LocalVariables|SetEndDistance (Math|Vector|VectorLength (- (Spline|GetLocationatTime _playerspline (LocalVariables|GetEnd) "World" _constantvelocity) _returnvalue)))
  (if (< (LocalVariables|GetStartDistance) (LocalVariables|GetEndDistance))
    (if (<= (LocalVariables|GetNum) 0)
      (LocalVariables|SetBest (LocalVariables|GetStart) :!label _label)
      (else
        (LocalVariables|SetNum (- (LocalVariables|GetNum) 1))
        (if (<= (LocalVariables|GetStartDistance) (Variables|Spline|GetDistanceThreshold))
          (goto _label)
          (else
            (bind _besttime (Spline|RecursiveDistanceCheck (LocalVariables|GetNum) (LocalVariables|GetStart) (Math|Float|Lerp (LocalVariables|GetStart) (LocalVariables|GetEnd) 0.5)))
            (LocalVariables|SetBest _besttime)))))
    (elif (<= (LocalVariables|GetNum) 0)
      (LocalVariables|SetBest (LocalVariables|GetEnd) :!label _label_2)
      (else
        (LocalVariables|SetNum (- (LocalVariables|GetNum) 1))
        (if (<= (LocalVariables|GetEndDistance) (Variables|Spline|GetDistanceThreshold))
          (goto _label_2)
          (else
            (bind _besttime_2 (Spline|RecursiveDistanceCheck (LocalVariables|GetNum) (Math|Float|Lerp (LocalVariables|GetStart) (LocalVariables|GetEnd) 0.5) (LocalVariables|GetEnd)))
            (LocalVariables|SetBest _besttime_2))))))
  (return (LocalVariables|GetBest)))

(fn UpdateDesiredTime
  (if (>= (Math|Float|Absolute(Float) (- (Variables|Spline|GetSplineDesiredTime) (Variables|Spline|GetSplineCurrentTime))) (Variables|Spline|GetTimeDifferenceThreshold))
    (Variables|Spline|SetSplineCurrentTime (Variables|Spline|GetSplineDesiredTime))
    (else
      (Variables|Spline|SetSplineCurrentTime (+ (* (- (Variables|Spline|GetSplineDesiredTime) (Variables|Spline|GetSplineCurrentTime)) (* (Variables|Default|GetDeltaTime) (Variables|Camera|GetCameraSpeed))) (Variables|Spline|GetSplineCurrentTime)))))
  (Variables|Camera|SetCameraDesiredLocation (Spline|GetLocationatTime (Variables|Spline|GetCameraSpline) (Variables|Spline|GetSplineCurrentTime) "World" (Variables|Spline|GetConstantVelocity))))

(fn DrawSplineDebug
  (params (Spline :type Spline%20Component%20Object%20Reference) (DesiredTime :type Float%20%28single-precision%29) (ConstantVelocity :type Boolean) (Color :type Linear%20Color%20Structure))
  (Rendering|Debug|DrawDebugSphere (Spline|GetLocationatTime Spline DesiredTime "World" ConstantVelocity) 5e+01 12 Color 0.0))