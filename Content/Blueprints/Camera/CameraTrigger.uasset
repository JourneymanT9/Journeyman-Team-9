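; Camera trigger actor that makes itself the ThirdPersonCharacter's active spline when that character overlaps it, including at BeginPlay.
; It passes itself and a transition time to the character's SetActiveSpline.
; A timeline then lerps the character's X and Y direction vectors from their current values to the trigger's own, re-orienting its axes gradually.
; Any end overlap stops that blend where it is, without checking which actor left.
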(event `self.ReceiveBeginPlay`
  (bind _returnvalue (`GameplayStatics.GetPlayerPawn` 0))
  ;[1 1 1] On beign play, If the player is overlapping then set this to be the active spline
  (if (`self.IsOverlappingActor` _returnvalue)
    (bind _asthird_person_character (cast `/Game/Blueprints/Character/ThirdPersonCharacter` _returnvalue))
    (`/Game/Blueprints/Character/ThirdPersonCharacter.SetActiveSpline` _asthird_person_character self (`self.TransitionTime`))
    (`self.SetDirectionAxis` _asthird_person_character (`/Game/Blueprints/Character/ThirdPersonCharacter.CharDirectionX` _asthird_person_character) (`/Game/Blueprints/Character/ThirdPersonCharacter.CharDirectionY` _asthird_person_character))))

(event `self.ReceiveActorBeginOverlap`
  (params (OtherActor :type "Actor Object Reference"))
  ;[1 1 1] On Overlap Begin, If the actor is the player then set this to be the active spline
  (bind _asthird_person_character (cast `/Game/Blueprints/Character/ThirdPersonCharacter` OtherActor))
  (`/Game/Blueprints/Character/ThirdPersonCharacter.SetActiveSpline` _asthird_person_character self (`self.TransitionTime`))
  (`self.SetDirectionAxis` _asthird_person_character (`/Game/Blueprints/Character/ThirdPersonCharacter.CharDirectionX` _asthird_person_character) (`/Game/Blueprints/Character/ThirdPersonCharacter.CharDirectionY` _asthird_person_character)))

(event `self.ReceiveTick`
  (params (DeltaSeconds :type "Float (single-precision)"))
  (`parent.ReceiveTick` DeltaSeconds))

(event `SetDirectionAxis`
  (params (Player :type "/Game/Blueprints/Character/ThirdPersonCharacter Object Reference") (StartDirX :type "Vector Structure") (StartDirY :type "Vector Structure"))
  (set `self.StartXAxis` StartDirX)
  (set `self.StartYAxis` StartDirY)
  (bind (_direction _alpha) (`Timeline|0-1` :!via `PlayFromStart` :!label _label)
    (:`Update`
      (set `/Game/Blueprints/Character/ThirdPersonCharacter.CharDirectionX` (`KismetMathLibrary.VLerp` (`self.StartXAxis`) (`self.CharDirectionX`) _alpha) Player)
      (set `/Game/Blueprints/Character/ThirdPersonCharacter.CharDirectionY` (`KismetMathLibrary.VLerp` (`self.StartYAxis`) (`self.CharDirectionY`) _alpha) Player))))

(event `self.ReceiveActorEndOverlap`
  (params (OtherActor :type "Actor Object Reference"))
  (goto _label :!via `Stop`))

(fn `UserConstructionScript`
  (`parent.UserConstructionScript`))